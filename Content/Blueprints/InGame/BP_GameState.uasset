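; BP_GameState is a game state that briefly shows a HUD widget, relayed through events named as client-to-server and server-to-multicast calls.
; On BeginPlay it caches the BP_HUD of player controller 0.
; CallWidget passes through C2S_SetWidgetVisibilty to S2M_SetWidgetVisibilty, which makes the widget visible on that cached HUD and hides it again after a short delay.
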(event `self.ReceiveBeginPlay`
  (bind _asbp_player_controller (cast `/Game/Blueprints/InGame/Character/Player/BP_PlayerController` (`GameplayStatics.GetPlayerController` 0)))
  (bind _asbp_hud (cast `/Game/Blueprints/InGame/BP_HUD` (`PlayerController.GetHUD` _asbp_player_controller)))
  (set `self.As BP HUD` _asbp_hud))

(event `CallWidget`
  (`self.C2S_SetWidgetVisibilty`))

(event `C2S_SetWidgetVisibilty`
  (`self.S2M_SetWidgetVisibilty`))

(event `S2M_SetWidgetVisibilty`
  (`/Game/Blueprints/InGame/BP_HUD.SetWidgetVisibility` (`self.As BP HUD`) true)
  (`KismetSystemLibrary.Delay` 3.0)
  (`/Game/Blueprints/InGame/BP_HUD.SetWidgetVisibility` (`self.As BP HUD`) false))

(fn `UserConstructionScript`)