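; Player controller that turns Enhanced Input actions into movement, camera look, jump, crouch and sprint on the possessed BP_Player.
; On BeginPlay it caches the pawn and, for the local player, adds the default mapping context, stores the HUD and sets game-only input.
; Movement follows control rotation, with forward flattened to yaw.
; Crouch toggles through a FlipFlop, while sprint is held and forwarded to the pawn's CallSprint.
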(event `self.ReceiveBeginPlay`
  (`WidgetBlueprintLibrary.SetInputMode_GameOnly` (`GameplayStatics.GetPlayerController` 0))
  (bind _asbp_player (cast `/Game/Blueprints/InGame/Character/Player/BP_Player` (`self.K2_GetPawn`)))
  (set `self.PlayerRef` _asbp_player)
  (if (`self.IsLocalPlayerController`)
    (`EnhancedInputSubsystemInterface.AddMappingContext` (subsystem `EnhancedInputLocalPlayerSubsystem`) "/Game/Input/IMC_Default.IMC_Default" 0 (struct))
    (bind _asbp_hud (cast `/Game/Blueprints/InGame/BP_HUD` (`self.GetHUD`)))
    (set `self.HUDRef` _asbp_hud)
    (`WidgetBlueprintLibrary.SetInputMode_GameOnly` null)))

(event `EnhancedInput|/Game/Input/Actions/IA_Move`
  (params (ActionValue :type "Vector2D Structure") (ElapsedSeconds :type "Float (double-precision)") (TriggeredSeconds :type "Float (double-precision)") (InputAction :type "InputAction Object Reference" :default "/Game/Input/Actions/IA_Move.IA_Move"))
  (bind (_returnvalue_roll _returnvalue_pitch _returnvalue_yaw) (`KismetMathLibrary.BreakRotator` (`self.GetControlRotation`)))
  (bind (_returnvalue_roll_2 _returnvalue_pitch_2 _returnvalue_yaw_2) (`KismetMathLibrary.BreakRotator` (`self.GetControlRotation`)))
  (bind _playerref (`self.PlayerRef`))
  (:`Triggered`
    (`|ExecutionSequence`
      (:`then_0`
        (`Pawn.AddMovementInput` _playerref (`KismetMathLibrary.GetRightVector` (`KismetMathLibrary.MakeRotator` _returnvalue_roll_2 0.0 _returnvalue_yaw_2)) ActionValue_X false))
      (:`then_1`
        (`Pawn.AddMovementInput` _playerref (`KismetMathLibrary.GetForwardVector` (`KismetMathLibrary.MakeRotator` 0.0 0.0 _returnvalue_yaw)) ActionValue_Y false)))))

(event `EnhancedInput|/Game/Input/Actions/IA_Jump`
  (params (ActionValue :type Boolean) (ElapsedSeconds :type "Float (double-precision)") (TriggeredSeconds :type "Float (double-precision)") (InputAction :type "InputAction Object Reference" :default "/Game/Input/Actions/IA_Jump.IA_Jump"))
  (bind _playerref (`self.PlayerRef`))
  (:`Triggered`
    (`Character.Jump` _playerref))
  (:`Canceled`
    (`Character.StopJumping` _playerref :!label _label))
  (:`Completed`
    (goto _label)))

(event `EnhancedInput|/Game/Input/Actions/IA_Look`
  (params (ActionValue :type "Vector2D Structure") (ElapsedSeconds :type "Float (double-precision)") (TriggeredSeconds :type "Float (double-precision)") (InputAction :type "InputAction Object Reference" :default "/Game/Input/Actions/IA_Look.IA_Look"))
  (:`Triggered`
    (`self.AddYawInput` ActionValue_X)
    (`self.AddPitchInput` ActionValue_Y)))

(event `EnhancedInput|/Game/Input/Actions/IA_Crouch`
  (params (ActionValue :type Boolean) (ElapsedSeconds :type "Float (double-precision)") (TriggeredSeconds :type "Float (double-precision)") (InputAction :type "InputAction Object Reference" :default "/Game/Input/Actions/IA_Crouch.IA_Crouch"))
  (bind _playerref (`self.PlayerRef`))
  (:`Started`
    (`/Engine/EditorBlueprintResources/StandardMacros.FlipFlop`
      (:`A`
        (`Character.Crouch` _playerref))
      (:`B`
        (`Character.UnCrouch` _playerref)))))

(event `EnhancedInput|/Game/Input/Actions/IA_Sprint`
  (params (ActionValue :type Boolean) (ElapsedSeconds :type "Float (double-precision)") (TriggeredSeconds :type "Float (double-precision)") (InputAction :type "InputAction Object Reference" :default "/Game/Input/Actions/IA_Sprint.IA_Sprint"))
  (bind _playerref (`self.PlayerRef`))
  (:`Triggered`
    (`/Game/Blueprints/InGame/Character/Player/BP_Player.CallSprint` _playerref true))
  (:`Canceled`
    (`/Game/Blueprints/InGame/Character/Player/BP_Player.CallSprint` _playerref false :!label _label_2))
  (:`Completed`
    (goto _label_2)))

(fn `UserConstructionScript`)