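; Player character Blueprint that handles sprinting and a timed damage-notice HUD widget, using paired C2S and S2M events named for client-to-server and multicast relay.
; CallSprint passes through C2S_Sprint, which picks sprint or walk speed for S2M_Sprint to apply to CharacterMovement.
; The damage notice follows the same relay, briefly showing the widget on player controller 0's BP_HUD.
; S2M_WidgetUpdate is an empty stub.
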(event `CallSprint`
  (params (bIsSprint :type Boolean))
  (`self.C2S_Sprint` bIsSprint))

(event `C2S_Sprint`
  (params (bIsSprint :type Boolean))
  (if bIsSprint
    (`self.S2M_Sprint` (`self.SprintSpeed`))
    (else
      (`self.S2M_Sprint` (`self.WalkSpeed`)))))

(event `S2M_Sprint`
  (params (WalkSpeed :type "Float (double-precision)"))
  (set `CharacterMovementComponent.MaxWalkSpeed` WalkSpeed (`self.CharacterMovement`)))

(event `C2S_DamageNoticeWidget`
  (`self.S2M_DamageNoticeWidget`))

(event `S2M_DamageNoticeWidget`
  (bind _asbp_hud (cast `/Game/Blueprints/InGame/BP_HUD` (`PlayerController.GetHUD` (`GameplayStatics.GetPlayerController` 0))))
  (`/Game/Blueprints/InGame/BP_HUD.SetWidgetVisibility` _asbp_hud true)
  (`KismetSystemLibrary.Delay` 4.0)
  (`/Game/Blueprints/InGame/BP_HUD.SetWidgetVisibility` _asbp_hud false))

(fn `S2M_WidgetUpdate`)

(fn `UserConstructionScript`
  (`parent.UserConstructionScript`))