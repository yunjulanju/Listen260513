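; BP_NPC is an in-game NPC character that switches between idle, crouch and jump states.
; SetIdleState maps a passed-in random integer to the next state, offering Idle in place of Jump when the NPC is crouched.
; SetStateAction then calls UnCrouch, Crouch or Jump for that state, resetting to Idle right after a jump.
; The event graph holds only disabled default events, so nothing here calls SetIdleState.
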(fn `SetIdleState`
  (params (RandomInt :type Integer))
  (if (`|EnumEquality` (`self.CurrentState`) "NewEnumerator2")
    (set `self.CurrentState` (select `int` (`local.RandomInt`) :`0` (enumliteral `/Game/Blueprints/Enum/E_State` "NewEnumerator0") :`1` "NewEnumerator2" :`2` "NewEnumerator0"))
    (else
      (set `self.CurrentState` (select `int` (`local.RandomInt`) :`0` (enumliteral `/Game/Blueprints/Enum/E_State` "NewEnumerator0") :`1` "NewEnumerator2" :`2` "NewEnumerator4"))))
  (`self.SetStateAction`))

(fn `SetStateAction`
  (switch `/Game/Blueprints/Enum/E_State` (`self.CurrentState`)
    (:`NewEnumerator0`
      (`self.UnCrouch`))
    (:`NewEnumerator2`
      (`self.Crouch`))
    (:`NewEnumerator4`
      (`self.Jump`)
      (set `self.CurrentState` "NewEnumerator0"))))

(fn `UserConstructionScript`
  (`parent.UserConstructionScript`))