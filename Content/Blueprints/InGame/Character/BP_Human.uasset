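; BP_Human is a character with health that drives a HUD health bar and ragdolls when health runs out.
; BeginPlay caches controller, HUD and game state, then sets the bar, which OnRep_HP refreshes as HP replicates.
; AnyDamage clamps HP and calls S2M_HitAction, which at zero HP disables movement and capsule collision and turns on mesh physics.
; That event's IsDead argument actually carries "still alive", so its inverted check triggers the ragdoll correctly.
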(event `self.ReceiveBeginPlay`
  (`|ExecutionSequence`
    (:`then_0`
      (bind _asbp_player_controller (cast `/Game/Blueprints/InGame/Character/Player/BP_PlayerController` (`self.GetController`)))
      (bind _output_get (set `self.PlayerControllerRef` _asbp_player_controller))
      (bind _asbp_hud (cast `/Game/Blueprints/InGame/BP_HUD` (`PlayerController.GetHUD` _output_get)))
      (set `self.HUDRef` _asbp_hud)
      (bind _asbp_game_state (cast `/Game/Blueprints/InGame/BP_GameState` (`GameplayStatics.GetGameState`)))
      (set `self.GameStateRef` _asbp_game_state))
    (:`then_1`
      (`/Engine/EditorBlueprintResources/StandardMacros.IsValid` (`self.HUDRef`)
        (:`Is Valid`
          (`/Game/Blueprints/UI/WBP_HP.SetPersent` (`/Game/Blueprints/InGame/BP_HUD.HPWidget` (`self.HUDRef`)) (/ (`self.HP`) (`self.MaxHP`))))))))

(event `self.ReceiveAnyDamage`
  (params (Damage :type "Float (single-precision)") (DamageType :type "DamageType Object Reference") (InstigatedBy :type "Controller Object Reference") (DamageCauser :type "Actor Object Reference"))
  (set `self.HP` (`KismetMathLibrary.FClamp` (- (`self.HP`) Damage) 0.0 (`self.MaxHP`)))
  (`self.S2M_HitAction` (> (`self.HP`) 0.0)))

(event `S2M_HitAction`
  (params (bIsDead :type Boolean))
  (bind _mesh (`self.Mesh`))
  (if (not bIsDead)
    (`CharacterMovementComponent.DisableMovement` (`self.CharacterMovement`))
    (`PrimitiveComponent.SetCollisionEnabled` (`self.CapsuleComponent`) "NoCollision")
    (`PrimitiveComponent.SetCollisionEnabled` _mesh "PhysicsOnly")
    (`PrimitiveComponent.SetSimulatePhysics` _mesh true)))

(fn `OnRep_HP`
  (bind _hudref (`self.HUDRef`))
  (`/Engine/EditorBlueprintResources/StandardMacros.IsValid` _hudref
    (:`Is Valid`
      (`/Game/Blueprints/UI/WBP_HP.SetPersent` (`/Game/Blueprints/InGame/BP_HUD.HPWidget` _hudref) (/ (`self.HP`) (`self.MaxHP`))))))

(fn `UserConstructionScript`)