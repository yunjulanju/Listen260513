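; BP_Trap is an environment trap that damages BP_Human actors that overlap its Box component.
; On BeginPlay it traces straight down on the Visibility channel and moves itself to the hit point, snapping onto the surface below.
; Damage is a small fixed amount applied only with authority; the c2s_Hit event is an empty, unused stub.
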(event `self.ReceiveBeginPlay`
  (bind (_returnvalue_x _returnvalue_y _returnvalue_z) (`KismetMathLibrary.BreakVector` (`self.K2_GetActorLocation`)))
  (bind (_outhit _returnvalue) (`KismetSystemLibrary.LineTraceSingle` (`KismetMathLibrary.MakeVector` _returnvalue_x _returnvalue_y _returnvalue_z) (`KismetMathLibrary.MakeVector` _returnvalue_x _returnvalue_y (- _returnvalue_z 10000.0)) "TraceTypeQuery1"))
  (if _returnvalue
    (`self.K2_SetActorLocation` (`.Location` (`GameplayStatics.BreakHitResult` _outhit)))))

(event `self.Box.OnComponentBeginOverlap`
  (params (OverlappedComponent :type "PrimitiveComponent Object Reference") (OtherActor :type "Actor Object Reference") (OtherComp :type "PrimitiveComponent Object Reference") (OtherBodyIndex :type Integer) (bFromSweep :type Boolean) (SweepResult :type "HitResult Structure (by ref)"))
  (bind _asbp_human (cast `/Game/Blueprints/InGame/Character/BP_Human` OtherActor))
  (`/Engine/EditorBlueprintResources/ActorMacros.Switch Has Authority`
    (:`Authority`
      (`GameplayStatics.ApplyDamage` _asbp_human 1.0))))

(event `c2s_Hit`
  (params (`BPHuman ` :type "/Game/Blueprints/InGame/Character/BP_Human Object Reference")))

(fn `UserConstructionScript`)